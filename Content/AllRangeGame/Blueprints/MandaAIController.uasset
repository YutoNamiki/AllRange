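; MandaAIController is the AI controller that drives a Manda pawn through MandaBehaviorTree.
; BeginPlay sets up MandaBlackboard with the default action state.
; A DoOnce on Tick defers the remaining setup to the first frame: it attaches the controller to its pawn, stores the pawn's location as HomeLocation and starts the tree.
; Tick also polls Life and destroys both pawn and controller when it is false.
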(event EventBeginPlay
  (Class|AIController|UseBlackboard "/Game/AllRangeGame/AI/MandaBlackboard.MandaBlackboard")
  (AI|Components|Blackboard|SetValueasEnum (Variables|Default|GetBlackboard) (Variables|Default|GetActionState) (Variables|Default|GetDefaultActionState)))

(event EventTick
  (params (DeltaSeconds :type Float%20%28single-precision%29))
  (bind _returnvalue (Pawn|GetControlledPawn))
  (Utilities|FlowControl|Sequence
    (:then_0
      (Utilities|FlowControl|DoOnce false
        (:Completed
          (Utilities|FlowControl|Sequence
            (:then_0
              (Class|Actor|AttachRootComponenttoActor _returnvalue "None" "KeepRelativeOffset" true)
              (AI|Components|Blackboard|SetValueasVector (Variables|Default|GetBlackboard) (Variables|Default|GetHomeLocation) (Transformation|GetActorLocation _returnvalue)))
            (:then_1
              (AI|RunBehaviorTree "/Game/AllRangeGame/AI/MandaBehaviorTree.MandaBehaviorTree"))))))
    (:then_1
      (if (not (Variables|Default|GetLife))
        (Actor|DestroyActor (Pawn|GetControlledPawn))
        (Actor|DestroyActor)))))

(fn ConstructionScript)