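; Enemy pawn that appears at its spawn time and rides a referenced spline, either looping until its survival time ends or until it reaches the end.
; The server advances distance and stores the transform for remotes to apply, destroying the spline when its reference count hits zero.
; Damage drains hit points; death awards points to the shooting player controller, freezes path movement and destroys the pawn after a hit.
; A sensor plays audio while a truck overlaps.
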(event OnComponentEndOverlap(AudioSensor)
  (params (OtherActor :type Actor%20Object%20Reference) (OtherComp :type Primitive%20Component%20Object%20Reference) (OtherBodyIndex :type Integer))
  (Utilities|Casting|CastToTruckActor OtherActor)
  (Audio|Components|Audio|Stop (Variables|Default|GetAudio)))

(event OnComponentBeginOverlap(AudioSensor)
  (params (OtherActor :type Actor%20Object%20Reference) (OtherComp :type Primitive%20Component%20Object%20Reference) (OtherBodyIndex :type Integer) (bFromSweep :type Boolean) (SweepResult :type Hit%20Result%20Structure%20%28by%20ref%29))
  (Utilities|Casting|CastToTruckActor OtherActor)
  (Audio|Components|Audio|Play (Variables|Default|GetAudio) 0.0))

(event OnComponentHit(Collision)
  (params (OtherActor :type Actor%20Object%20Reference) (OtherComp :type Primitive%20Component%20Object%20Reference) (NormalImpulse :type Vector :default "0, 0, 0") (Hit :type Hit%20Result%20Structure%20%28by%20ref%29))
  (if (Variables|Default|GetDead)
    (Utilities|FlowControl|Delay 3.0)
    (Actor|DestroyActor)))

(event Game|Damage|EventAnyDamage
  (params (Damage :type Float%20%28single-precision%29) (DamageType :type Damage%20Type%20Object%20Reference) (InstigatedBy :type Controller%20Object%20Reference) (DamageCauser :type Actor%20Object%20Reference))
  (bind _output_get (Variables|Default|SetHitPoint (- (Variables|Default|GetHitPoint) (Math|Float|Truncate Damage))))
  (if (<= _output_get 0)
    (bind _asarrow_shooting_player_controller (Utilities|Casting|CastToArrowShootingPlayerController InstigatedBy))
    (Variables|/Game/AllRangeGame/Blueprints/ArrowShootingPlayerController.ArrowShootingPlayerController_C|SetPoint _asarrow_shooting_player_controller (+ (Variables|/Game/AllRangeGame/Blueprints/ArrowShootingPlayerController.ArrowShootingPlayerController_C|GetPoint _asarrow_shooting_player_controller) (Variables|Default|GetPoint)))
    (Variables|Default|SetDead true)
    (else
      (Variables|Default|SetDamaged true))))

(event EventBeginPlay
  (Rendering|SetVisibility (Variables|Default|GetSkeletalMesh) false false))

(event EventTick
  (params (DeltaSeconds :type Float%20%28single-precision%29))
  (bind _spline (Variables|Default|GetSpline))
  (bind _spline_2 (Variables|Default|GetSpline))
  (bind _spline_3 (Variables|Default|GetSpline))
  (bind _spline_4 (Variables|/Game/AllRangeGame/Blueprints/SplineActor.SplineActor_C|GetSpline _spline))
  (bind _returnvalue (Spline|GetSplineLength _spline_4))
  (bind _output_get (Variables|Default|SetDeltaTime DeltaSeconds))
  (Variables|Default|SetElapsedTime (+ _output_get (Variables|Default|GetElapsedTime)))
  (if (>= (Utilities|Time|GetRealTimeSeconds) (Variables|Default|GetSpawnTime))
    (Utilities|FlowControl|Sequence
      (:then_0
        (Utilities|FlowControl|DoOnce false
          (:Completed
            (Rendering|SetVisibility (Variables|Default|GetSkeletalMesh) true false)
            (Variables|Default|SetMoving true))))
      (:then_1
        (if (not (Variables|Default|GetArrived))
          (Networking|SwitchHasAuthority
            (:Authority
              (if (Variables|Default|GetDead)
                (Variables|Default|SetLocation (Transformation|GetActorLocation))
                (Variables|Default|SetRotation (Transformation|GetActorRotation))
                (elif (Variables|Default|GetLoop)
                  (if (> (Variables|Default|GetSpeed) 0.0)
                    (Variables|Default|SetMoveDistance (+ (Variables|Default|GetMoveDistance) (* (Variables|Default|GetDeltaTime) (Variables|Default|GetSpeed))))
                    (else
                      (Variables|Default|SetMoveDistance (+ (+ (Variables|Default|GetMoveDistance) (* (Variables|Default|GetDeltaTime) (Variables|Default|GetSpeed))) (Spline|GetSplineLength (Variables|/Game/AllRangeGame/Blueprints/SplineActor.SplineActor_C|GetSpline (Variables|Default|GetSpline)))))))
                  (bind (_location _direction _rotation) (Default|GetCurrentLocationandRotation (Variables|Default|GetSpline) (Variables|Default|GetMoveDistance) true))
                  (Transformation|SetActorLocationAndRotation _location _rotation)
                  (Variables|Default|SetLocation _location)
                  (Variables|Default|SetRotation _rotation)
                  (if (>= (Variables|Default|GetElapsedTime) (+ (Variables|Default|GetSurvivalTime) (Variables|Default|GetSpawnTime)))
                    (Actor|DestroyActor)
                    (bind _result (Math|Integer|DecrementInt (Variables|/Game/AllRangeGame/Blueprints/SplineActor.SplineActor_C|GetReferencedCount _spline_3))
                      (:%20%20
                        (if (== _result 0)
                          (Actor|DestroyActor _spline_3)))))
                  (else
                    (if (> (Variables|Default|GetSpeed) 0.0)
                      (Variables|Default|SetMoveDistance (+ (Variables|Default|GetMoveDistance) (* (Variables|Default|GetDeltaTime) (Variables|Default|GetSpeed))))
                      (else
                        (Variables|Default|SetMoveDistance (+ (+ (Variables|Default|GetMoveDistance) (* (Variables|Default|GetDeltaTime) (Variables|Default|GetSpeed))) (Spline|GetSplineLength (Variables|/Game/AllRangeGame/Blueprints/SplineActor.SplineActor_C|GetSpline (Variables|Default|GetSpline)))))))
                    (if (>= (Variables|Default|GetMoveDistance) _returnvalue)
                      (Variables|Default|SetMoveDistance _returnvalue)
                      (Variables|Default|SetArrived true)
                      (bind (_location_2 _direction_2 _rotation_2) (Default|GetCurrentLocationandRotation (Variables|Default|GetSpline) (Variables|Default|GetMoveDistance) true))
                      (Transformation|SetActorLocationAndRotation _location_2 _rotation_2)
                      (Variables|Default|SetLocation _location_2)
                      (Variables|Default|SetRotation _rotation_2)
                      (Actor|DestroyActor)
                      (bind _result_2 (Math|Integer|DecrementInt (Variables|/Game/AllRangeGame/Blueprints/SplineActor.SplineActor_C|GetReferencedCount _spline_2))
                        (:%20%20
                          (if (== _result_2 0)
                            (Actor|DestroyActor _spline_2))))
                      (else
                        (bind (_location_3 _direction_3 _rotation_3) (Default|GetCurrentLocationandRotation (Variables|Default|GetSpline) (Variables|Default|GetMoveDistance) true))
                        (Transformation|SetActorLocationAndRotation _location_3 _rotation_3)
                        (Variables|Default|SetLocation _location_3)
                        (Variables|Default|SetRotation _rotation_3)))))))
            (:Remote
              (Transformation|SetActorLocationAndRotation (Variables|Default|GetLocation) (Variables|Default|GetRotation)))))))))

(fn ConstructionScript
  (bind _spline (Variables|Default|GetSpline))
  (Utilities|IsValid _spline
    (:Is%20Valid
      (bind (_location _direction _rotation) (Default|GetCurrentLocationandRotation _spline 0.0 true))
      (Transformation|SetActorLocationAndRotation _location _rotation))))

(fn Moveto
  (params (TargetLocation :type Vector) (ScaleValue :type Float%20%28single-precision%29))
  (Pawn|Input|AddMovementInput (Math|Vector|Normalize (- TargetLocation (Transformation|GetActorLocation))) ScaleValue true))

(fn Rotateto
  (params (TargetLocation :type Vector))
  (Transformation|SetActorRotation (Math|Rotator|Lerp(Rotator) (Transformation|GetActorRotation) (Math|Rotator|FindLookatRotation (Transformation|GetActorLocation) TargetLocation) 0.1 true)))