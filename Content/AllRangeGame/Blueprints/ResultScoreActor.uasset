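; ResultScoreActor displays an integer result score as a row of 3D digit meshes.
; Tick waits until Value is not -1, then DoOnce builds the number a single time.
; CountDigits finds the length by powers of ten, and SetNumberMesh adds a static mesh component per digit with the shared MaterialInstance.
; The row is offset along X by NumberWidth, centring odd digit counts but leaving even counts off-centre.
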(event EventBeginPlay)

(event Collision|EventActorBeginOverlap
  (params (OtherActor :type Actor%20Object%20Reference)))

(event EventTick
  (params (DeltaSeconds :type Float%20%28single-precision%29))
  (if (!= (Variables|Default|GetValue) -1)
    (Utilities|FlowControl|DoOnce false
      (:Completed
        (CallFunction|SetNumberMesh (Variables|Default|GetValue) (CallFunction|CountDigits (Variables|Default|GetValue)) (Variables|Default|GetNumberWidth) (Variables|Default|GetMaterialInstance))))))

(fn ConstructionScript)

(fn CountDigits
  (params (CountValue :type Integer))
  (bind _digitsnum (LocalVariables|GetdigitsNum))
  (while (> (/ CountValue (Math|Float|Truncate (Math|Float|Power 1e+01 (Math|Conversions|ToFloat(Integer) (LocalVariables|GetdigitsNum))))) 0)
    (Math|Integer|IncrementInt _digitsnum))
  (return _digitsnum))

(fn SetNumberMesh
  (params (Value :type Integer) (DigitsCount :type Integer) (NumberWidth :type Float%20%28single-precision%29) (MaterialInstance :type Material%20Instance%20Object%20Reference))
  (bind _returnvalue (/ DigitsCount 2))
  (bind _returnvalue_2 (* _returnvalue NumberWidth))
  (if (== (Math|Integer|%(Integer) DigitsCount 2) 0)
    (LocalVariables|SetinitialLocation (Math|Vector|MakeVector (* (+ _returnvalue_2 (/ NumberWidth 2.0)) -1.0) 0.0 0.0))
    (else
      (LocalVariables|SetinitialLocation (Math|Vector|MakeVector (* _returnvalue_2 -1.0) 0.0 0.0))))
  (for _index (range 0 (- DigitsCount 1))
    (bind _returnvalue_3 (AddComponent|AddStaticMeshComponent false (Math|Transform|MakeTransform (+ (Math|Vector|MakeVector (* _index NumberWidth) 0.0 0.0) (LocalVariables|GetinitialLocation)))))
    (switch int (Math|Integer|%(Integer) (/ Value (Math|Float|Truncate (Math|Float|Power 1e+01 (Math|Conversions|ToFloat(Integer) (- DigitsCount (+ _index 1)))))) 10)
      (:0
        (Components|StaticMesh|SetStaticMesh _returnvalue_3 "/Game/AllRangeGame/Meshes/count0.count0"))
      (:1
        (Components|StaticMesh|SetStaticMesh _returnvalue_3 "/Game/AllRangeGame/Meshes/count1.count1"))
      (:2
        (Components|StaticMesh|SetStaticMesh _returnvalue_3 "/Game/AllRangeGame/Meshes/count2.count2"))
      (:3
        (Components|StaticMesh|SetStaticMesh _returnvalue_3 "/Game/AllRangeGame/Meshes/count3.count3"))
      (:4
        (Components|StaticMesh|SetStaticMesh _returnvalue_3 "/Game/AllRangeGame/Meshes/count4.count4"))
      (:5
        (Components|StaticMesh|SetStaticMesh _returnvalue_3 "/Game/AllRangeGame/Meshes/count5.count5"))
      (:6
        (Components|StaticMesh|SetStaticMesh _returnvalue_3 "/Game/AllRangeGame/Meshes/count6.count6"))
      (:7
        (Components|StaticMesh|SetStaticMesh _returnvalue_3 "/Game/AllRangeGame/Meshes/count7.count7"))
      (:8
        (Components|StaticMesh|SetStaticMesh _returnvalue_3 "/Game/AllRangeGame/Meshes/count8.count8"))
      (:9
        (Components|StaticMesh|SetStaticMesh _returnvalue_3 "/Game/AllRangeGame/Meshes/count9.count9")))
    (Rendering|Material|SetMaterial _returnvalue_3 0 MaterialInstance)))