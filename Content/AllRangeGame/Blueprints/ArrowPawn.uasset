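; ArrowPawn is a projectile pawn that damages enemies it hits in the AllRangeGame.
; On collision hit it casts the other actor in turn to EnemyPawn, SplineEnemyPawn and MandaPawn, applying AttackValue damage credited to the firing player controller.
; A hit on any of these spawns an explosion emitter and destroys the arrow, while hitting anything else destroys it after a short delay.
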(event OnComponentHit(Collision)
  (params (OtherActor :type Actor%20Object%20Reference) (OtherComp :type Primitive%20Component%20Object%20Reference) (NormalImpulse :type Vector :default "0, 0, 0") (Hit :type Hit%20Result%20Structure%20%28by%20ref%29))
  (bind _self self)
  (bind _attackvalue (Variables|Default|GetAttackValue))
  (bind _firedplayercontroller (Variables|Default|GetFiredPlayerController))
  (bind _returnvalue (Math|Conversions|ToFloat(Integer) _attackvalue))
  (bind _asenemy_pawn (Utilities|Casting|CastToEnemyPawn OtherActor)
    (:then
      (Game|Damage|ApplyDamage _asenemy_pawn _returnvalue _firedplayercontroller _self)
      (Effects|SpawnEmitteratLocation "/Game/StarterContent/Particles/P_Explosion.P_Explosion" (Transformation|GetActorLocation) (Transformation|GetActorRotation) :!label _label)
      (Actor|DestroyActor))
    (:CastFailed
      (bind _asspline_enemy_pawn (Utilities|Casting|CastToSplineEnemyPawn OtherActor)
        (:then
          (Game|Damage|ApplyDamage _asspline_enemy_pawn _returnvalue _firedplayercontroller _self)
          (goto _label))
        (:CastFailed
          (bind _asmanda_pawn (Utilities|Casting|CastToMandaPawn OtherActor)
            (:then
              (Game|Damage|ApplyDamage _asmanda_pawn _returnvalue _firedplayercontroller _self)
              (goto _label))
            (:CastFailed
              (Utilities|FlowControl|Delay 3.0)
              (Actor|DestroyActor))))))))

(event EventBeginPlay)

(event EventTick
  (params (DeltaSeconds :type Float%20%28single-precision%29)))

(fn ConstructionScript)