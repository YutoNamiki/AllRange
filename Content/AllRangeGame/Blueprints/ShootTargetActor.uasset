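; ShootTargetActor is a target that reacts when an ArrowPawn strikes it.
; Both overlap and hit events on its Sphere component cast the other actor to ArrowPawn and share one response.
; A Hit flag, never reset here, limits it to a single trigger, playing the Rotate timeline from start to drive the static mesh's relative yaw while keeping roll and pitch.
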(event OnComponentBeginOverlap(Sphere)
  (params (OtherActor :type Actor%20Object%20Reference) (OtherComp :type Primitive%20Component%20Object%20Reference) (OtherBodyIndex :type Integer) (bFromSweep :type Boolean) (SweepResult :type Hit%20Result%20Structure%20%28by%20ref%29))
  (bind _staticmesh (Variables|Default|GetStaticMesh))
  (bind _relativerotation (Variables|/Script/Engine.SceneComponent|GetRelativeRotation _staticmesh))
  (bind (_roll _pitch) (Math|Rotator|BreakRotator _relativerotation))
  (Utilities|Casting|CastToArrowPawn OtherActor)
  (if (not (Variables|Default|GetbHit))
    (Variables|Default|SetbHit true)
    (bind _newrotate (Timeline|Rotate PlayFromStart)
      (:Update
        (Transformation|SetRelativeRotation _staticmesh (Math|Rotator|MakeRotator _roll _pitch _newrotate) false false)))))

(event OnComponentHit(Sphere)
  (params (OtherActor :type Actor%20Object%20Reference) (OtherComp :type Primitive%20Component%20Object%20Reference) (NormalImpulse :type Vector :default "0, 0, 0") (Hit :type Hit%20Result%20Structure%20%28by%20ref%29))
  (bind _staticmesh (Variables|Default|GetStaticMesh))
  (bind _relativerotation (Variables|/Script/Engine.SceneComponent|GetRelativeRotation _staticmesh))
  (bind (_roll _pitch) (Math|Rotator|BreakRotator _relativerotation))
  (Utilities|Casting|CastToArrowPawn OtherActor)
  (if (not (Variables|Default|GetbHit))
    (Variables|Default|SetbHit true)
    (bind _newrotate (Timeline|Rotate PlayFromStart)
      (:Update
        (Transformation|SetRelativeRotation _staticmesh (Math|Rotator|MakeRotator _roll _pitch _newrotate) false false)))))

(event EventBeginPlay)

(event EventActorBeginOverlap
  (params (OtherActor :type Actor%20Object%20Reference)))

(event EventTick
  (params (DeltaSeconds :type Float%20%28single-precision%29)))

(fn ConstructionScript)