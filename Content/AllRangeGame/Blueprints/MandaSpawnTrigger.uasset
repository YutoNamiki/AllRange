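; MandaSpawnTrigger is an actor that spawns AI-controllable MandaPawns once a TruckActor overlaps it.
; The overlap only sets a Triggered flag, which Tick checks on the authority side.
; While the flag is set, Tick spawns a pawn at the configured location, rotation and scale and gives it its default controller.
; Nothing here clears the flag, so spawning repeats every tick after the first truck overlap.
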(event EventBeginPlay)

(event EventActorBeginOverlap
  (params (OtherActor :type Actor%20Object%20Reference))
  (Utilities|Casting|CastToTruckActor OtherActor)
  (Variables|Default|SetbTriggered true))

(event EventTick
  (params (DeltaSeconds :type Float%20%28single-precision%29))
  (Networking|SwitchHasAuthority
    (:Authority
      (if (Variables|Default|GetbTriggered)
        (bind _returnvalue (Game|SpawnActorfromClass "/Game/AllRangeGame/Blueprints/MandaPawn.MandaPawn_C" (Math|Transform|MakeTransform (Variables|Default|GetSpawnLocation) (Variables|Default|GetSpawnRotation) (Variables|Default|GetSpawnScale)) "Undefined" 0 0))
        (Pawn|SpawnDefaultController _returnvalue)))))

(fn ConstructionScript)