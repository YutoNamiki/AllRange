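; Trigger actor that spawns timed waves of enemy pawns once the Truck overlaps its TriggerVolume.
; Tick latches the trigger, accumulates elapsed time and spawns each SpawnInformations entry when its AppearanceTime passes, removing it from the array inside the loop.
; SpawnEnemyPawn creates the pawn at the actor's location, sets its hit points and score value, and passes movement targets to its EnemyAIController.
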(event EventBeginPlay)

(event EventTick
  (params (DeltaSeconds :type Float%20%28single-precision%29))
  (if (Collision|IsOverlappingActor (Variables|Default|GetTruck) (Variables|Default|GetTriggerVolume) :!class /Script/Engine.Actor)
    (Variables|Default|SetIsTriggered true))
  (if (Variables|Default|GetIsTriggered)
    (Variables|Default|SetElapsedTime (+ DeltaSeconds (Variables|Default|GetElapsedTime)))
    (for (_array_element _array_index) (Variables|Default|GetSpawnInformations)
      (if (<= (.AppearanceTime (Utilities|Struct|BreakEnemySpawnInformation _array_element)) (Variables|Default|GetElapsedTime))
        (CallFunction|SpawnEnemyPawn (Transformation|GetActorLocation) (.MoveInformation (Utilities|Struct|BreakEnemySpawnInformation _array_element)) (.HP (Utilities|Struct|BreakEnemySpawnInformation _array_element)) (.Point (Utilities|Struct|BreakEnemySpawnInformation _array_element)) (Variables|Default|GetNavigation))
        (Utilities|Array|RemoveIndex (Variables|Default|GetSpawnInformations) _array_index)))))

(fn ConstructionScript)

(fn SpawnEnemyPawn
  (params (Location :type Vector) (SpawnInfo :type Array%20of%20Moving%20Target%20Point%20Information%20Structures) (HP :type Integer) (Point :type Integer) (Navigation :type Navigation%20Volume%20Object%20Reference))
  (bind _returnvalue (Game|SpawnActorfromClass (Variables|Default|GetSpawnPawn) (Math|Transform|MakeTransform Location) "Undefined" 0 0))
  (Pawn|SpawnDefaultController _returnvalue)
  (bind _asenemy_pawn (Utilities|Casting|CastToEnemyPawn _returnvalue))
  (Variables|/Game/AllRangeGame/Blueprints/EnemyPawn.EnemyPawn_C|SetHitPoint _asenemy_pawn HP)
  (Variables|/Game/AllRangeGame/Blueprints/EnemyPawn.EnemyPawn_C|SetPoint _asenemy_pawn Point)
  (bind _asenemy_aicontroller (Utilities|Casting|CastToEnemyAIController (Pawn|GetController _returnvalue)))
  (Default|SetTargetActors _asenemy_aicontroller SpawnInfo)
  (Variables|Default|SetNavigation Navigation))