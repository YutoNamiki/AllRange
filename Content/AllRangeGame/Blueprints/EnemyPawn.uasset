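; EnemyPawn is an enemy that moves with floating pawn movement and awards points to an ArrowShootingPlayerController when killed.
; MoveTo sets a direction that Tick applies until within range, while RotateTo eases rotation and SetMovementParameters tunes the movement component.
; Damage lowers hit points and flags Damaged or, for a kill credited to that controller, Dead.
; Dead enemies enable sphere physics and are destroyed three seconds after a hit.
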(event OnComponentHit(Sphere)
  (params (OtherActor :type Actor%20Object%20Reference) (OtherComp :type Primitive%20Component%20Object%20Reference) (NormalImpulse :type Vector :default "0, 0, 0") (Hit :type Hit%20Result%20Structure%20%28by%20ref%29))
  (if (Variables|Default|GetDead)
    (Utilities|FlowControl|Delay 3.0)
    (Actor|DestroyActor)))

(event Custom|AddMoveInput
  (Pawn|Input|AddMovementInput (Variables|Default|GetMoveDirection) 1.0 true))

(event Game|Damage|EventAnyDamage
  (params (Damage :type Float%20%28single-precision%29) (DamageType :type Damage%20Type%20Object%20Reference) (InstigatedBy :type Controller%20Object%20Reference) (DamageCauser :type Actor%20Object%20Reference))
  (bind _output_get (Variables|Default|SetHitPoint (- (Variables|Default|GetHitPoint) (Math|Float|Truncate Damage))))
  (if (<= _output_get 0)
    (bind _asarrow_shooting_player_controller (Utilities|Casting|CastToArrowShootingPlayerController InstigatedBy))
    (Variables|/Game/AllRangeGame/Blueprints/ArrowShootingPlayerController.ArrowShootingPlayerController_C|SetPoint _asarrow_shooting_player_controller (+ (Variables|/Game/AllRangeGame/Blueprints/ArrowShootingPlayerController.ArrowShootingPlayerController_C|GetPoint _asarrow_shooting_player_controller) (Variables|Default|GetPoint)))
    (Variables|Default|SetDead true)
    (else
      (Variables|Default|SetDamaged true))))

(event EventBeginPlay)

(event EventActorBeginOverlap
  (params (OtherActor :type Actor%20Object%20Reference)))

(event EventTick
  (params (DeltaSeconds :type Float%20%28single-precision%29))
  (if (Variables|Default|GetDead)
    (Physics|SetSimulatePhysics (Variables|Default|GetSphere) true)
    (elif (Variables|Default|GetMoving)
      (CallFunction|AddMoveInput))))

(fn ConstructionScript)

(fn Moveto
  (params (TargetLocation :type Vector) (DeterminationDistanceRange :type Float%20%28single-precision%29))
  (bind _returnvalue (Transformation|GetActorLocation))
  (if (>= DeterminationDistanceRange (Math|Vector|VectorLength (- TargetLocation _returnvalue)))
    (Variables|Default|SetMoveDirection "0, 0, 0")
    (Variables|Default|SetMoving false)
    (return true)
    (else
      (Variables|Default|SetMoveDirection (Class|KismetMathLibrary|GetDirectionVector _returnvalue TargetLocation))
      (Variables|Default|SetMoving true)
      (return false))))

(fn Rotateto
  (params (TargetRotation :type Rotator))
  (Transformation|SetActorRotation (Math|Rotator|Lerp(Rotator) TargetRotation (Transformation|GetActorRotation) 0.9 true)))

(fn SetMovementParameters
  (params (MaxSpeed :type Float%20%28single-precision%29) (Acceleration :type Float%20%28single-precision%29) (Deceleration :type Float%20%28single-precision%29) (TurningBoost :type Float%20%28single-precision%29))
  (bind _floatingpawnmovement (Variables|Default|GetFloatingPawnMovement))
  (Variables|/Script/Engine.FloatingPawnMovement|SetMaxSpeed _floatingpawnmovement MaxSpeed)
  (Variables|/Script/Engine.FloatingPawnMovement|SetAcceleration _floatingpawnmovement Acceleration)
  (Variables|/Script/Engine.FloatingPawnMovement|SetDeceleration _floatingpawnmovement Deceleration)
  (Variables|/Script/Engine.FloatingPawnMovement|SetTurningBoost _floatingpawnmovement TurningBoost))