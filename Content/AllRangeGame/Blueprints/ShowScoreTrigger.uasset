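; Results scoreboard actor for the arrow-shooting game that briefly displays a score, then destroys itself.
; ShowScore runs once, gathering players, copying controller points by player number and ranking them by repeatedly extracting the maximum.
; It spawns one ResultScoreActor using the first gathered player's points, not the sorted result, and reveals the board through server-to-multicast visibility events.
; Player board placement is unfinished: nothing here calls it, and most branches are disconnected.
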(event Custom|SortScore
  (bind _playernumber (Variables|Default|GetPlayerNumber))
  (bind _localpoint (Variables|Default|GetLocalpoint))
  (bind (_indexofmaxvalue _maxvalue) (Math|Integer|MaxOfIntArray _localpoint))
  ;[1 1 1] スコアのソート
  (while (> (Utilities|Array|Length (Variables|Default|GetLocalpoint)) 0)
    (Utilities|Array|Add (Variables|Default|GetLocalPointSorted) _maxvalue)
    (Utilities|Array|SetArrayElem (Variables|Default|GetPlayerRanking) (Variables|Default|GetIterator) (Utilities|Array|Get(acopy) _playernumber _indexofmaxvalue))
    (Utilities|Array|RemoveIndex _playernumber _indexofmaxvalue)
    (Utilities|Array|RemoveIndex _localpoint _indexofmaxvalue)
    (Math|Integer|IncrementInt (Variables|Default|GetIterator))))

(event Custom|SetVisibility_MultiCast
  (params (Visibility :type Boolean))
  (Rendering|SetVisibility (Variables|Default|GetScoreBoard1) Visibility false)
  (Rendering|SetVisibility (Variables|Default|GetScoreText1) Visibility false))

(event Custom|SetVisibility_Server
  (params (Visibility :type Boolean))
  (CallFunction|SetVisibilityMultiCast Visibility))

(event Custom|SetPlayerTextLocation_MultiCast
  (for (_array_element _array_index) (Variables|Default|GetPlayerRanking)
    (if (== _array_index 0)
      (Game|SpawnActorfromClass "/Game/AllRangeGame/Blueprints/Player1BoardActor.Player1BoardActor_C" (Transformation|GetWorldTransform (Variables|Default|Get1stScorePlayerTextPos)) "Undefined" 0 0))))

(event Custom|UpdateScore_Server
  ;[1 1 1] それぞれのプレイヤーのスコアとプレイヤーナンバーを配列に格納
  (for _array_element (Variables|Default|GetPlayers)
    (if (== (Variables|/Game/AllRangeGame/Blueprints/ArrowShootingPlayer.ArrowShootingPlayer_C|GetPlayerNumber _array_element) 1)
      (bind _asarrow_shooting_player_controller (Utilities|Casting|CastToArrowShootingPlayerController (Pawn|GetController _array_element)))
      (Utilities|Array|SetArrayElem (Variables|Default|GetLocalpoint) 0 (Variables|/Game/AllRangeGame/Blueprints/ArrowShootingPlayerController.ArrowShootingPlayerController_C|GetPoint _asarrow_shooting_player_controller))
      (Utilities|Array|SetArrayElem (Variables|Default|GetPlayerNumber) 0 1)
      (elif (== (Variables|/Game/AllRangeGame/Blueprints/ArrowShootingPlayer.ArrowShootingPlayer_C|GetPlayerNumber _array_element) 2)
        (bind _asarrow_shooting_player_controller_2 (Utilities|Casting|CastToArrowShootingPlayerController (Pawn|GetController _array_element)))
        (Utilities|Array|SetArrayElem (Variables|Default|GetLocalpoint) 1 (Variables|/Game/AllRangeGame/Blueprints/ArrowShootingPlayerController.ArrowShootingPlayerController_C|GetPoint _asarrow_shooting_player_controller_2))
        (Utilities|Array|SetArrayElem (Variables|Default|GetPlayerNumber) 1 2)
        (else
          (bind _asarrow_shooting_player_controller_3 (Utilities|Casting|CastToArrowShootingPlayerController (Pawn|GetController _array_element)))
          (Utilities|Array|SetArrayElem (Variables|Default|GetLocalpoint) 2 (Variables|/Game/AllRangeGame/Blueprints/ArrowShootingPlayerController.ArrowShootingPlayerController_C|GetPoint _asarrow_shooting_player_controller_3))
          (Utilities|Array|SetArrayElem (Variables|Default|GetPlayerNumber) 2 3))))))

(event Custom|SpawnScoreActor_Server
  (bind _1stscorevaluepos (Variables|Default|Get1stScoreValuePos))
  (bind _returnvalue (Transformation|GetWorldTransform _1stscorevaluepos))
  (bind (_location _rotation _scale) (Math|Transform|BreakTransform _returnvalue))
  (bind (_roll _pitch _yaw) (Math|Rotator|BreakRotator _rotation))
  (bind _returnvalue_2 (Game|SpawnActorfromClass "/Game/AllRangeGame/Blueprints/ResultScoreActor.ResultScoreActor_C" (Math|Transform|MakeTransform _location (Math|Rotator|MakeRotator _roll _pitch (- _yaw 9e+01)) _scale) "Undefined" 0 0))
  (bind _asarrow_shooting_player_controller (Utilities|Casting|CastToArrowShootingPlayerController (Pawn|GetController (Utilities|Array|Get(acopy) (Variables|Default|GetPlayers)))))
  (Variables|/Game/AllRangeGame/Blueprints/ResultScoreActor.ResultScoreActor_C|SetValue _returnvalue_2 (Variables|/Game/AllRangeGame/Blueprints/ArrowShootingPlayerController.ArrowShootingPlayerController_C|GetPoint _asarrow_shooting_player_controller))
  (Variables|/Game/AllRangeGame/Blueprints/ResultScoreActor.ResultScoreActor_C|SetMaterialInstance _returnvalue_2 (Utilities|Array|Get(acopy) (Variables|Default|GetMaterialInstance))))

(event Custom|GetPlayersReference_Server
  ;[1 1 1] プレイヤーへの参照を取得
  (bind _outactors (Actor|GetAllActorsOfClass "/Game/AllRangeGame/Blueprints/ArrowShootingPlayer.ArrowShootingPlayer_C"))
  (for _array_element _outactors
    (Utilities|Array|Add (Variables|Default|GetPlayers) _array_element)))

(event Custom|ShowScore
  (Utilities|FlowControl|DoOnce false
    (:Completed
      (CallFunction|GetPlayersReferenceServer)
      (CallFunction|UpdateScoreServer)
      (CallFunction|SortScore)
      (CallFunction|SpawnScoreActorServer)
      (CallFunction|SetVisibilityServer true)
      (Utilities|FlowControl|Delay (Variables|Default|GetSurvivalTime))
      (Actor|DestroyActor))))

(fn ConstructionScript
  (bind _scoreboard1pos (Variables|Default|GetScoreBoard1Pos))
  (bind _scoretext1pos (Variables|Default|GetScoreText1Pos))
  (bind _returnvalue (Transformation|GetWorldTransform _scoretext1pos))
  (bind _returnvalue_2 (Transformation|GetWorldTransform _scoreboard1pos))
  (bind (_location _rotation) (Math|Transform|BreakTransform _returnvalue))
  (bind (_location_2 _rotation_2) (Math|Transform|BreakTransform _returnvalue_2))
  (bind (_roll _pitch _yaw) (Math|Rotator|BreakRotator _rotation))
  (bind (_roll_2 _pitch_2 _yaw_2) (Math|Rotator|BreakRotator _rotation_2))
  ;[1 1 1] 正面を向くように設定
  (Transformation|SetWorldLocationAndRotation (Variables|Default|GetScoreBoard1) _location_2 (Math|Rotator|MakeRotator _roll_2 _pitch_2 (- _yaw_2 9e+01)) false false)
  (Transformation|SetWorldLocationAndRotation (Variables|Default|GetScoreText1) _location (Math|Rotator|MakeRotator _roll _pitch (- _yaw 9e+01)) false false))

(fn OnRepMaterialInstance)