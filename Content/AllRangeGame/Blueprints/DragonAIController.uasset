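; AI controller for a dragon enemy that sets up its blackboard and keeps target and path lists.
; On the first Tick, it attaches itself to the controlled pawn, initializes EnemyBlackboard and stores the pawn's location as HomeLocation plus a default ActionState.
; SetTargetActors stores the target list and writes its last entry to TargetObject; small helpers query both arrays.
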(event EventBeginPlay)

(event EventTick
  (params (DeltaSeconds :type Float%20%28single-precision%29))
  (Utilities|FlowControl|DoOnce false
    (:Completed
      (Class|Actor|AttachRootComponenttoActor (Pawn|GetControlledPawn) "None" "KeepRelativeOffset" true)
      (bind _blackboardcomponent (Class|AIController|UseBlackboard "/Game/AllRangeGame/AI/EnemyBlackboard.EnemyBlackboard"))
      (Variables|Default|SetBlackboard_1 _blackboardcomponent)
      (Utilities|FlowControl|Sequence
        (:then_0
          (AI|Components|Blackboard|SetValueasVector (Variables|Default|GetBlackboard_1) (Variables|Default|GetHomeLocation) (Transformation|GetActorLocation (Pawn|GetControlledPawn))))
        (:then_1
          (AI|Components|Blackboard|SetValueasEnum (Variables|Default|GetBlackboard_1) (Variables|Default|GetActionState) (Variables|Default|GetDefaultActionState)))))))

(fn ConstructionScript)

(fn HasPath
  (return (> (Utilities|Array|Length (Variables|Default|GetPath)) 0)))

(fn HasTargetActors
  (return (> (Utilities|Array|Length (Variables|Default|GetTargetActors)) 0)))

(fn GetLastIndexinPath
  (bind _path (Variables|Default|GetPath))
  (return (Utilities|Array|Get(acopy) _path (Utilities|Array|LastIndex _path))))

(fn GetLastIndexinTargetActors
  (bind _targetactors (Variables|Default|GetTargetActors))
  (return (Utilities|Array|Get(acopy) _targetactors (Utilities|Array|LastIndex _targetactors))))

(fn SetTargetActors
  (params (TargetActors :type Array%20of%20Actor%20Object%20References))
  (Variables|Default|SetTargetActors TargetActors)
  (AI|Components|Blackboard|SetValueasObject (Variables|Default|GetBlackboard_1) (Variables|Default|GetTargetObject) (CallFunction|GetLastIndexinTargetActors)))

(fn GetFirstIndexinTargetActors
  (return (Utilities|Array|Get(acopy) (Variables|Default|GetTargetActors))))