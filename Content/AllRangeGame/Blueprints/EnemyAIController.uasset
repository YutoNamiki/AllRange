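; AI controller for enemy pawns in the AllRange game, holding a movement Path and a list of TargetInfos with per-target movement settings.
; Helper functions report whether path or targets exist and return the last entry of each, including its speed, acceleration, deceleration and turning values.
; MoveTo, RotateTo and SetMovementParameters forward to the controlled EnemyPawn.
; On first Tick it attaches itself to that pawn.
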(event EventBeginPlay)

(event EventTick
  (params (DeltaSeconds :type Float%20%28single-precision%29))
  (Utilities|FlowControl|DoOnce false
    (:Completed
      (Class|Actor|AttachRootComponenttoActor (Pawn|GetControlledPawn) "None" "KeepRelativeOffset" true))))

(fn ConstructionScript)

(fn HasPath
  (return (> (Utilities|Array|Length (Variables|Default|GetPath)) 0)))

(fn HasTargetActors
  (return (> (Utilities|Array|Length (Variables|Default|GetTargetInfos)) 0)))

(fn GetLastIndexinTargetActors
  (bind _targetinfos (Variables|Default|GetTargetInfos))
  (return (.TargetActor (Utilities|Struct|BreakMovingTargetPointInformation (Utilities|Array|Get(acopy) _targetinfos (Utilities|Array|LastIndex _targetinfos))))))

(fn GetLastIndexinPath
  (bind _path (Variables|Default|GetPath))
  (return (Utilities|Array|Get(acopy) _path (Utilities|Array|LastIndex _path))))

(fn Moveto
  (params (TargetLocation :type Vector) (DeterminationDistanceRange :type Float%20%28single-precision%29))
  (bind _asenemy_pawn (Utilities|Casting|CastToEnemyPawn (Pawn|GetControlledPawn))
    (:then
      (bind _isarrived (Default|Moveto _asenemy_pawn TargetLocation DeterminationDistanceRange))
      (return _isarrived))
    (:CastFailed
      (return false))))

(fn Rotateto
  (params (TargetRotation :type Rotator))
  (bind _asenemy_pawn (Utilities|Casting|CastToEnemyPawn (Pawn|GetControlledPawn)))
  (Default|Rotateto _asenemy_pawn TargetRotation))

(fn SetMovementParameters
  (params (MaxSpeed :type Float%20%28single-precision%29) (Acceleration :type Float%20%28single-precision%29) (Deceleration :type Float%20%28single-precision%29) (TurningBoost :type Float%20%28single-precision%29))
  (bind _asenemy_pawn (Utilities|Casting|CastToEnemyPawn (Pawn|GetControlledPawn)))
  (Default|SetMovementParameters _asenemy_pawn MaxSpeed Acceleration Deceleration TurningBoost))

(fn GetLastIndexinMovementParameters
  (bind _targetinfos (Variables|Default|GetTargetInfos))
  (bind _returnvalue (Utilities|Array|LastIndex _targetinfos))
  (bind _item (Utilities|Array|Get(acopy) _targetinfos _returnvalue))
  (bind (_targetactor _maxmovespeed _moveacceleration _movedeceleration _turningboost) (Utilities|Struct|BreakMovingTargetPointInformation _item))
  (return _maxmovespeed _moveacceleration _movedeceleration _turningboost))