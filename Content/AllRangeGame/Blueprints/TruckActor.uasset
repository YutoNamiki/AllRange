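; Truck actor that travels a looping spline in a networked game and offers threat points to pawns.
; On Tick the authority advances distance by speed and derives the lap count, while remotes only reposition from MoveDistance, both offset along the spline's up vector.
; Overlapping a TruckSpeedChanger changes speed once its target lap minus one is reached.
; GetNearestThreatPoint searches components cached at BeginPlay for the closest usable, unoccupied one.
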(event Custom|OnMoveSplineServer
  (params (DeltaTime :type Float%20%28single-precision%29))
  (bind _spline (Variables|スプライン|GetSpline))
  (bind _spline_2 (Variables|/Game/AllRangeGame/Blueprints/SplineActor.SplineActor_C|GetSpline _spline))
  (bind _returnvalue (Spline|GetSplineLength _spline_2))
  (if (> (Variables|スプライン|GetSpeed) 0.0)
    (Variables|スプライン|SetMoveDistance (+ (* DeltaTime (Variables|スプライン|GetSpeed)) (Variables|スプライン|GetMoveDistance)))
    (else
      (Variables|スプライン|SetMoveDistance (+ (+ (* DeltaTime (Variables|スプライン|GetSpeed)) (Variables|スプライン|GetMoveDistance)) _returnvalue))))
  (Variables|スプライン|SetLap (Math|Float|Truncate (/ (Variables|スプライン|GetMoveDistance) _returnvalue)))
  (bind (_location _direction _rotation) (Default|GetCurrentLocationandRotation (Variables|スプライン|GetSpline) (Variables|スプライン|GetMoveDistance) true))
  (Transformation|SetActorLocationAndRotation (+ _location (* (Math|Vector|GetUpVector _rotation) (Variables|スプライン|GetHeightOffset))) _rotation true))

(event EventBeginPlay
  (Variables|ウェイポイント|SetThreatPoints (Actor|GetComponentsByClass "/Game/AllRangeGame/Blueprints/ThreatPointComponent.ThreatPointComponent_C")))

(event EventActorBeginOverlap
  (params (OtherActor :type Actor%20Object%20Reference))
  (bind _astruck_speed_changer (Utilities|Casting|CastToTruckSpeedChanger OtherActor))
  (if (>= (Variables|スプライン|GetLap) (- (Variables|/Game/AllRangeGame/Blueprints/TruckSpeedChanger.TruckSpeedChanger_C|GetTargetLap _astruck_speed_changer) 1))
    (Variables|スプライン|SetSpeed (Variables|/Game/AllRangeGame/Blueprints/TruckSpeedChanger.TruckSpeedChanger_C|GetChangeSpeed _astruck_speed_changer))))

(event EventTick
  (params (DeltaSeconds :type Float%20%28single-precision%29))
  (if (Variables|スプライン|GetbMove)
    (Networking|SwitchHasAuthority
      (:Authority
        (CallFunction|OnMoveSplineServer DeltaSeconds))
      (:Remote
        (bind (_location _direction _rotation) (Default|GetCurrentLocationandRotation (Variables|スプライン|GetSpline) (Variables|スプライン|GetMoveDistance) true))
        (Transformation|SetActorLocationAndRotation (+ _location (* (Math|Vector|GetUpVector _rotation) (Variables|スプライン|GetHeightOffset))) _rotation true)))))

(fn ConstructionScript)

(fn GetNearestThreatPoint
  (params (FindingPawn :type Pawn%20Object%20Reference))
  (for (_array_element _array_index) (Variables|ウェイポイント|GetThreatPoints)
    (if (and (Variables|/Game/AllRangeGame/Blueprints/ThreatPointComponent.ThreatPointComponent_C|GetCanUse _array_element) (not (Variables|/Game/AllRangeGame/Blueprints/ThreatPointComponent.ThreatPointComponent_C|GetIsUsing _array_element)))
      (if (< (LocalVariables|Getdistance) 0.0)
        (LocalVariables|SetnearestPointIndex _array_index)
        (LocalVariables|Setdistance (Math|Vector|VectorLength (- (Transformation|GetWorldLocation _array_element) (Transformation|GetActorLocation FindingPawn))))
        (elif (<= (Math|Vector|VectorLength (- (Transformation|GetWorldLocation _array_element) (Transformation|GetActorLocation FindingPawn))) (LocalVariables|Getdistance))
          (LocalVariables|SetnearestPointIndex _array_index)
          (LocalVariables|Setdistance (Math|Vector|VectorLength (- (Transformation|GetWorldLocation _array_element) (Transformation|GetActorLocation FindingPawn))))))))
  (if (!= (LocalVariables|GetnearestPointIndex) -1)
    (return (!= (LocalVariables|GetnearestPointIndex) -1) (Utilities|Array|Get(acopy) (Variables|ウェイポイント|GetThreatPoints) (LocalVariables|GetnearestPointIndex)))
    (else
      (return (!= (LocalVariables|GetnearestPointIndex) -1) 0))))