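; CameraLibrary provides a helper function that returns the player's camera location, with or without VR.
; With a head-mounted display enabled, GetCameraLocation un-rotates the device position by the device rotation, then transforms it by the player 0 camera manager's actor transform.
; Otherwise it returns that manager's camera location, or the zero vector when the manager is invalid.
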(fn GetCameraLocation
  (params (SelfActor :type Actor%20Object%20Reference))
  (bind _returnvalue (Game|GetPlayerCameraManager SelfActor))
  (bind (_devicerotation _deviceposition) (Class|HeadMountedDisplayFunctionLibrary|GetOrientationandPosition))
  (Utilities|IsValid _returnvalue
    (:Is%20Valid
      (if (Class|HeadMountedDisplayFunctionLibrary|IsHeadMountedDisplayEnabled)
        ;[1 1 1] VR
        (bind _output_get (LocalVariables|SetOutLocation (Math|Transform|TransformLocation (Transformation|GetActorTransform (Game|GetPlayerCameraManager SelfActor)) (Math|Vector|UnrotateVector _deviceposition _devicerotation))))
        (return _output_get)
        (else
          ;[1 1 1] No VR
          (bind _output_get_2 (LocalVariables|SetOutLocation (Camera|GetCameraLocation _returnvalue)))
          (return _output_get_2))))
    (:Is%20Not%20Valid
      (bind _output_get_3 (LocalVariables|SetOutLocation "0, 0, 0"))
      (return _output_get_3))))