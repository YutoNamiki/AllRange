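; MandaPawn is a damageable target pawn that awards points to the ArrowShootingPlayerController that hits it.
; AnyDamage lowers HitPoint, then grants BonusPoint if the damage causer overlaps either bonus box, otherwise normal Point.
; When HitPoint runs out, it grants KnockDownBonusPoint instead and sets Dead.
; Each award spawns a ScoreActor oriented by the first TruckActor's location, if one exists, and animates it vertically with a timeline.
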(event EventBeginPlay)

(event EventActorBeginOverlap
  (params (OtherActor :type Actor%20Object%20Reference)))

(event EventTick
  (params (DeltaSeconds :type Float%20%28single-precision%29)))

(event Game|Damage|EventAnyDamage
  (params (Damage :type Float%20%28single-precision%29) (DamageType :type Damage%20Type%20Object%20Reference) (InstigatedBy :type Controller%20Object%20Reference) (DamageCauser :type Actor%20Object%20Reference))
  (bind _returnvalue (Transformation|GetActorLocation))
  (bind _returnvalue_2 (Transformation|GetActorLocation))
  (bind _returnvalue_3 (Transformation|GetActorLocation))
  (bind _returnvalue_4 (+ _returnvalue "0,0.000000,50.000000"))
  (bind _returnvalue_5 (+ _returnvalue_2 "0,0.000000,50.000000"))
  (bind _returnvalue_6 (+ _returnvalue_3 "0,0.000000,50.000000"))
  (bind _output_get (Variables|Default|SetHitPoint (- (Variables|Default|GetHitPoint) (Math|Float|Truncate Damage))))
  (bind _asarrow_shooting_player_controller (Utilities|Casting|CastToArrowShootingPlayerController InstigatedBy))
  (if (> _output_get 0)
    (if (or (Collision|IsOverlappingActor (Variables|コンポーネント|GetBonusBox) DamageCauser :!class /Script/Engine.PrimitiveComponent) (Collision|IsOverlappingActor (Variables|コンポーネント|GetBonusBox1) DamageCauser :!class /Script/Engine.PrimitiveComponent))
      (Variables|/Game/AllRangeGame/Blueprints/ArrowShootingPlayerController.ArrowShootingPlayerController_C|SetPoint _asarrow_shooting_player_controller (+ (Variables|/Game/AllRangeGame/Blueprints/ArrowShootingPlayerController.ArrowShootingPlayerController_C|GetPoint _asarrow_shooting_player_controller) (Variables|Default|GetBonusPoint)))
      (bind _outactors (Actor|GetAllActorsOfClass "/Game/AllRangeGame/Blueprints/TruckActor.TruckActor_C"))
      (Utilities|IsValid (Utilities|Array|Get(acopy) _outactors)
        (:Is%20Valid
          (bind _returnvalue_7 (Game|SpawnActorfromClass "/Game/AllRangeGame/Blueprints/ScoreActor.ScoreActor_C" (Math|Transform|MakeTransform _returnvalue_5 (Math|Rotator|CombineRotators "0,-90.000000, 0" (Math|Rotator|FindLookatRotation _returnvalue_5 (Transformation|GetActorLocation (Utilities|Array|Get(acopy) _outactors))))) "Undefined" 0 0))
          (Variables|/Game/AllRangeGame/Blueprints/ScoreActor.ScoreActor_C|SetValue _returnvalue_7 (Variables|Default|GetBonusPoint))
          (bind _offset (Timeline|AppearanceMove_1 Play)
            (:Update
              (Transformation|AddActorWorldOffset _returnvalue_7 (Math|Vector|MakeVector 0.0 0.0 _offset))))))
      (else
        (Variables|/Game/AllRangeGame/Blueprints/ArrowShootingPlayerController.ArrowShootingPlayerController_C|SetPoint _asarrow_shooting_player_controller (+ (Variables|/Game/AllRangeGame/Blueprints/ArrowShootingPlayerController.ArrowShootingPlayerController_C|GetPoint _asarrow_shooting_player_controller) (Variables|Default|GetPoint)))
        (bind _outactors_2 (Actor|GetAllActorsOfClass "/Game/AllRangeGame/Blueprints/TruckActor.TruckActor_C"))
        (Utilities|IsValid (Utilities|Array|Get(acopy) _outactors_2)
          (:Is%20Valid
            (bind _returnvalue_8 (Game|SpawnActorfromClass "/Game/AllRangeGame/Blueprints/ScoreActor.ScoreActor_C" (Math|Transform|MakeTransform _returnvalue_6 (Math|Rotator|CombineRotators "0,-90.000000, 0" (Math|Rotator|FindLookatRotation _returnvalue_6 (Transformation|GetActorLocation (Utilities|Array|Get(acopy) _outactors_2))))) "Undefined" 0 0))
            (Variables|/Game/AllRangeGame/Blueprints/ScoreActor.ScoreActor_C|SetValue _returnvalue_8 (Variables|Default|GetPoint))
            (bind _offset_2 (Timeline|AppearanceMove_2 Play)
              (:Update
                (Transformation|AddActorWorldOffset _returnvalue_8 (Math|Vector|MakeVector 0.0 0.0 _offset_2))))))))
    (else
      (Variables|/Game/AllRangeGame/Blueprints/ArrowShootingPlayerController.ArrowShootingPlayerController_C|SetPoint _asarrow_shooting_player_controller (+ (Variables|/Game/AllRangeGame/Blueprints/ArrowShootingPlayerController.ArrowShootingPlayerController_C|GetPoint _asarrow_shooting_player_controller) (Variables|Default|GetKnockDownBonusPoint)))
      (Variables|Default|SetDead true)
      (bind _outactors_3 (Actor|GetAllActorsOfClass "/Game/AllRangeGame/Blueprints/TruckActor.TruckActor_C"))
      (Utilities|IsValid (Utilities|Array|Get(acopy) _outactors_3)
        (:Is%20Valid
          (bind _returnvalue_9 (Game|SpawnActorfromClass "/Game/AllRangeGame/Blueprints/ScoreActor.ScoreActor_C" (Math|Transform|MakeTransform _returnvalue_4 (Math|Rotator|CombineRotators "0,-90.000000, 0" (Math|Rotator|FindLookatRotation _returnvalue_4 (Transformation|GetActorLocation (Utilities|Array|Get(acopy) _outactors_3))))) "Undefined" 0 0))
          (Variables|/Game/AllRangeGame/Blueprints/ScoreActor.ScoreActor_C|SetValue _returnvalue_9 (Variables|Default|GetKnockDownBonusPoint))
          (bind _offset_3 (Timeline|AppearanceMove_3 Play)
            (:Update
              (Transformation|AddActorWorldOffset _returnvalue_9 (Math|Vector|MakeVector 0.0 0.0 _offset_3)))))))))

(fn ConstructionScript)