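; Spline rail actor that builds a visible track along its spline and answers path queries by distance.
; The construction script labels each control point with its index in text hidden in game.
; It lays a RailMesh spline mesh on each segment flagged in the Visible array, which it pads with true entries.
; Helper functions return world location, direction and rotation at a distance, optionally looped, and report when a distance reaches the spline's end.
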(event EventBeginPlay)

(event EventActorBeginOverlap
  (params (OtherActor :type Actor%20Object%20Reference)))

(event EventTick
  (params (DeltaSeconds :type Float%20%28single-precision%29)))

(fn ConstructionScript
  (bind _spline (Variables|Default|GetSpline))
  (bind _spline_2 (Variables|Default|GetSpline))
  ;[1 1 1] 制御点のインデックスを表示させる
  (for _index (range 0 (- (Spline|GetNumberOfSplinePoints (Variables|Default|GetSpline)) 1))
    (bind _rotation (CallFunction|GetCurrentLocationandRotation (Spline|GetDistanceAlongSplineatSplinePoint _spline _index) false))
    (bind _returnvalue (AddComponent|AddTextRenderComponent false (Math|Transform|MakeTransform (.Location (Spline|GetLocationandTangentatSplinePoint _spline _index "Local")) _rotation)))
    (Rendering|Components|TextRender|SetText _returnvalue (Utilities|Text|ToText(Integer) _index))
    (Rendering|Components|TextRender|SetXScale _returnvalue 3.0)
    (Rendering|Components|TextRender|SetYScale _returnvalue 3.0)
    (Development|SetHiddeninGame _returnvalue true false)
    (if (< (Utilities|Array|Length (Variables|Default|GetbVisible)) (- (Spline|GetNumberOfSplinePoints (Variables|Default|GetSpline)) 1))
      (Utilities|Array|Add (Variables|Default|GetbVisible) true)))
  ;[1 1 1] Splineに沿ったメッシュ作成
  (for _index_2 (range 0 (- (Spline|GetNumberOfSplinePoints (Variables|Default|GetSpline)) 2))
    (if (Utilities|Array|Get(acopy) (Variables|Default|GetbVisible) _index_2)
      (bind _returnvalue_2 (AddComponent|AddSplineMeshComponent false))
      (Components|StaticMesh|SetStaticMesh _returnvalue_2 (Variables|Default|GetRailMesh))
      (SplineMesh|SetStartandEnd _returnvalue_2 (.Location (Spline|GetLocationandTangentatSplinePoint _spline_2 _index_2 "Local")) (.Tangent (Spline|GetLocationandTangentatSplinePoint _spline_2 _index_2 "Local")) (.Location (Spline|GetLocationandTangentatSplinePoint _spline_2 (+ _index_2 1) "Local")) (.Tangent (Spline|GetLocationandTangentatSplinePoint _spline_2 (+ _index_2 1) "Local")) :!class /Script/Engine.SplineMeshComponent))))

(fn GetCurrentLocationandRotation
  (params (Length :type Float%20%28single-precision%29) (Loop :type Boolean))
  (bind _spline (Variables|Default|GetSpline))
  (if Loop
    (LocalVariables|SetlocalLength (Math|Float|%(Float) Length (Spline|GetSplineLength (Variables|Default|GetSpline))))
    (else
      (LocalVariables|SetlocalLength Length)))
  (return (Spline|GetLocationatDistanceAlongSpline _spline (LocalVariables|GetlocalLength) "World") (Spline|GetDirectionatDistanceAlongSpline _spline (LocalVariables|GetlocalLength) "World") (Spline|GetRotationatDistanceAlongSpline _spline (LocalVariables|GetlocalLength) "World")))

(fn IsArrived
  (params (Length :type Float%20%28single-precision%29))
  (return (>= Length (Spline|GetSplineLength (Variables|Default|GetSpline)))))