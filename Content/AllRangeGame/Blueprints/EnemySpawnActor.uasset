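; EnemySpawnActor is a timed spawner that creates enemy pawns at its own location according to a list of spawn entries.
; Tick accumulates elapsed time, spawns a pawn for each entry whose appearance time has passed, and removes that entry from the list within the loop.
; SpawnEnemyPawn gives each pawn its default controller, casts it to DragonAIController, and hands over the entry's move targets and the Navigation reference.
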(event EventBeginPlay)

(event EventActorBeginOverlap
  (params (OtherActor :type Actor%20Object%20Reference)))

(event EventTick
  (params (DeltaSeconds :type Float%20%28single-precision%29))
  (Variables|Default|SetElapsedTime (+ DeltaSeconds (Variables|Default|GetElapsedTime)))
  (for (_array_element _array_index) (Variables|Default|GetSpawnInformations)
    (if (<= (.AppearanceTime (Utilities|Struct|BreakEnemySpawnInformation _array_element)) (Variables|Default|GetElapsedTime))
      (CallFunction|SpawnEnemyPawn (Transformation|GetActorLocation) (.MoveInformation (Utilities|Struct|BreakEnemySpawnInformation _array_element)) (Variables|Default|GetNavigation))
      (Utilities|Array|RemoveIndex (Variables|Default|GetSpawnInformations) _array_index))))

(fn ConstructionScript)

(fn SpawnEnemyPawn
  (params (Location :type Vector) (SpawnInfo :type Array%20of%20Moving%20Target%20Point%20Information%20Structures) (Navigation :type Navigation%20Volume%20Object%20Reference))
  (bind _returnvalue (Game|SpawnActorfromClass (Variables|Default|GetSpawnPawn) (Math|Transform|MakeTransform Location) "Undefined" 0 0))
  (Pawn|SpawnDefaultController _returnvalue)
  (bind _asdragon_aicontroller (Utilities|Casting|CastToDragonAIController (Pawn|GetController _returnvalue)))
  (Default|SetTargetActors _asdragon_aicontroller SpawnInfo)
  (Variables|/Game/AllRangeGame/Blueprints/DragonAIController.DragonAIController_C|SetNavigation _asdragon_aicontroller Navigation))