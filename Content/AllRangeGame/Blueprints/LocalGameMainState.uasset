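; LocalGameMainState is a state Blueprint that marks when a match in AllRangeGame starts, once all expected players have joined.
; On Tick, the authority side sets the Gaming flag once IsAllPlayersJoined succeeds, and nothing here clears it.
; That check counts ArrowShootingPlayerController actors against PlayerCount on LocalGameMainMode, returning false if the game mode cast fails.
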(event EventBeginPlay)

(event EventTick
  (params (DeltaSeconds :type Float%20%28single-precision%29))
  (Networking|SwitchHasAuthority
    (:Authority
      (if (and (CallFunction|IsAllPlayersJoined) (not (Variables|Default|GetGaming)))
        (Variables|Default|SetGaming true)))))

(fn ConstructionScript)

(fn IsAllPlayersJoined
  (bind _aslocal_game_main_mode (Utilities|Casting|CastToLocalGameMainMode (Game|GetGameMode))
    (:then
      (bind _outactors (Actor|GetAllActorsOfClass "/Game/AllRangeGame/Blueprints/ArrowShootingPlayerController.ArrowShootingPlayerController_C"))
      (return (== (Utilities|Array|Length _outactors) (Variables|/Game/AllRangeGame/Blueprints/LocalGameMainMode.LocalGameMainMode_C|GetPlayerCount _aslocal_game_main_mode))))
    (:CastFailed
      (return false))))