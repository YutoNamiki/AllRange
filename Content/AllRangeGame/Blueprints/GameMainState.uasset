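; GameMainState tracks when the multiplayer arrow-shooting game starts by setting a Gaming flag once all players have joined.
; Every Tick on the authority, IsAllPlayersJoined compares the number of ArrowShootingPlayerController actors with PlayerCount from MultiplayGameMode.
; The flag is only ever set to true here, and the join check returns false if the game mode cast fails.
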(event EventBeginPlay)

(event EventTick
  (params (DeltaSeconds :type Float%20%28single-precision%29))
  (Networking|SwitchHasAuthority
    (:Authority
      (if (and (CallFunction|IsAllPlayersJoined) (not (Variables|Default|GetGaming)))
        (Variables|Default|SetGaming true)))))

(fn ConstructionScript)

(fn IsAllPlayersJoined
  (bind _asmultiplay_game_mode (Utilities|Casting|CastToMultiplayGameMode (Game|GetGameMode))
    (:then
      (bind _outactors (Actor|GetAllActorsOfClass "/Game/AllRangeGame/Blueprints/ArrowShootingPlayerController.ArrowShootingPlayerController_C"))
      (return (== (Utilities|Array|Length _outactors) (Variables|/Game/AllRangeGame/Blueprints/GameMainMode.GameMainMode_C|GetPlayerCount _asmultiplay_game_mode))))
    (:CastFailed
      (return false))))