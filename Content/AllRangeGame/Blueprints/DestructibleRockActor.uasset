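; DestructibleRockActor is an actor with a destructible component that blows apart on a timer and then removes itself.
; A DoOnce on Tick starts a single sequence: after a short delay, it applies massive radius damage with a strong impulse.
; The damage originates behind the component along its negative forward vector.
; After a longer delay the actor destroys itself.
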(event EventBeginPlay)

(event EventActorBeginOverlap
  (params (OtherActor :type Actor%20Object%20Reference)))

(event EventTick
  (params (DeltaSeconds :type Float%20%28single-precision%29))
  (bind _destructiblecomponent (Variables|Default|GetDestructibleComponent))
  (Utilities|FlowControl|DoOnce false
    (:Completed
      (Utilities|FlowControl|Delay 5.3)
      (Class|DestructibleComponent|ApplyRadiusDamage _destructiblecomponent 5e+04 (+ (Transformation|GetWorldLocation _destructiblecomponent) (* (* (Math|Vector|GetForwardVector _destructiblecomponent) -1.0) 5e+02)) 5e+04 1e+06 false)
      (Utilities|FlowControl|Delay 2e+01)
      (Actor|DestroyActor))))

(fn ConstructionScript)