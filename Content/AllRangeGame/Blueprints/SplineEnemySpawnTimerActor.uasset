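; Timer actor that spawns SplineEnemyPawns at a target spline's actor location from a timed SpawnInformation list.
; BeginPlay raises the spline's ReferencedCount once per entry.
; Tick accumulates time on the authority and spawns each due entry whose required PlayerCount the GameMainMode meets, passing spline, movement, lifetime and point settings.
; Spawned entries leave the list, and the actor destroys itself when removal empties it.
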(event EventBeginPlay
  (bind _targetspline (Variables|Default|GetTargetSpline))
  (for _array_element (Variables|Default|GetSpawnInformation)
    (bind _result (Math|Integer|IncrementInt (Variables|/Game/AllRangeGame/Blueprints/SplineActor.SplineActor_C|GetReferencedCount _targetspline))
      (:%20%20
        (Variables|/Game/AllRangeGame/Blueprints/SplineActor.SplineActor_C|SetReferencedCount _targetspline _result)))))

(event EventActorBeginOverlap
  (params (OtherActor :type Actor%20Object%20Reference)))

(event EventTick
  (params (DeltaSeconds :type Float%20%28single-precision%29))
  (bind _spawninformation (Variables|Default|GetSpawnInformation))
  (Networking|SwitchHasAuthority
    (:Authority
      (Variables|Default|SetElapsedTime (+ DeltaSeconds (Variables|Default|GetElapsedTime)))
      (for (_array_element _array_index) (Variables|Default|GetSpawnInformation)
        (if (<= (.SpawnTime (Utilities|Struct|BreakSplineEnemySpawnInformation _array_element)) (Variables|Default|GetElapsedTime))
          (bind _asgame_main_mode (Utilities|Casting|CastToGameMainMode (Game|GetGameMode)))
          (if (>= (Variables|/Game/AllRangeGame/Blueprints/GameMainMode.GameMainMode_C|GetPlayerCount _asgame_main_mode) (.PlayerCount (Utilities|Struct|BreakSplineEnemySpawnInformation _array_element)))
            (CallFunction|SpawnSplineEnemyPawn (Transformation|GetActorLocation (Variables|Default|GetTargetSpline)) (Variables|Default|GetTargetSpline) (.SurvivalTime (Utilities|Struct|BreakSplineEnemySpawnInformation _array_element)) (.Speed (Utilities|Struct|BreakSplineEnemySpawnInformation _array_element)) (.Loop (Utilities|Struct|BreakSplineEnemySpawnInformation _array_element)) (.HitPoint (Utilities|Struct|BreakSplineEnemySpawnInformation _array_element)) (.Point (Utilities|Struct|BreakSplineEnemySpawnInformation _array_element)))
            (Utilities|Array|RemoveIndex _spawninformation _array_index)
            (if (== (Utilities|Array|Length _spawninformation) 0)
              (Actor|DestroyActor))))))))

(fn ConstructionScript)

(fn SpawnSplineEnemyPawn
  (params (Location :type Vector) (TargetSpline :type Spline%20Actor%20Object%20Reference) (SurvivalTime :type Float%20%28single-precision%29) (Speed :type Float%20%28single-precision%29) (Loop :type Boolean) (Point :type Integer) (HitPoint :type Integer))
  (bind _returnvalue (Game|SpawnActorfromClass "/Game/AllRangeGame/Blueprints/SplineEnemyPawn.SplineEnemyPawn_C" (Math|Transform|MakeTransform Location) "Undefined" 0 0))
  (Variables|/Game/AllRangeGame/Blueprints/SplineEnemyPawn.SplineEnemyPawn_C|SetSpline _returnvalue TargetSpline)
  (Variables|/Game/AllRangeGame/Blueprints/SplineEnemyPawn.SplineEnemyPawn_C|SetSurvivalTime _returnvalue SurvivalTime)
  (Variables|/Game/AllRangeGame/Blueprints/SplineEnemyPawn.SplineEnemyPawn_C|SetSpeed _returnvalue Speed)
  (Variables|/Game/AllRangeGame/Blueprints/SplineEnemyPawn.SplineEnemyPawn_C|SetLoop _returnvalue Loop)
  (Variables|/Game/AllRangeGame/Blueprints/SplineEnemyPawn.SplineEnemyPawn_C|SetHitPoint _returnvalue Point)
  (Variables|/Game/AllRangeGame/Blueprints/SplineEnemyPawn.SplineEnemyPawn_C|SetPoint _returnvalue HitPoint))